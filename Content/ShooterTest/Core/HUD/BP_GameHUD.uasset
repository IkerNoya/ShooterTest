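; BP_GameHUD manages the player UI and death screen for the shooter game.
; On BeginPlay it waits a tick, caches BP_GameMode, creates both W_Player and W_DeathScreen with that reference, shows the player UI and sets game-only input.
; It binds to the game mode's OnLoose event, which swaps the player UI for the death screen, shows the cursor and switches to UI-only input.
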(event Custom|Loose
  (bind _returnvalue (Game|GetPlayerController 0))
  (Widget|RemovefromParent (Variables|Default|GetPlayerUI))
  (UserInterface|Viewport|AddtoViewport (Variables|Default|GetDeathUI) 0)
  (Variables|/Script/Engine.PlayerController|SetbShowMouseCursor _returnvalue true)
  (Input|SetInputModeUIOnly _returnvalue 0 "DoNotLock"))

(event EventBeginPlay
  (bind _returnvalue (Game|GetPlayerController 0))
  (Utilities|FlowControl|Delay 0.0)
  (bind _asbp_game_mode (Utilities|Casting|CastToBP_GameMode (Game|GetGameMode)))
  (Variables|Default|SetGameMode _asbp_game_mode)
  (bind _returnvalue_2 (UserInterface|CreateWidget "/Game/ShooterTest/UI/W_Player.W_Player_C" (Game|GetPlayerController 0) _asbp_game_mode))
  (bind _output_get (Variables|Default|SetPlayerUI _returnvalue_2))
  (UserInterface|Viewport|AddtoViewport _output_get 0)
  (bind _returnvalue_3 (UserInterface|CreateWidget "/Game/ShooterTest/UI/W_DeathScreen.W_DeathScreen_C" 0 (Variables|Default|GetGameMode)))
  (Variables|Default|SetDeathUI _returnvalue_3)
  (EventDispatchers|BindEventtoOnLoose (Variables|Default|GetGameMode) (delegate Custom|Loose))
  (Variables|/Script/Engine.PlayerController|SetbShowMouseCursor _returnvalue false)
  (Input|SetInputModeGameOnly _returnvalue))

(fn ConstructionScript)