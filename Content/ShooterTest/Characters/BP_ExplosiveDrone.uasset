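; BP_ExplosiveDrone is a drone character that explodes when it attacks or dies.
; Attack plays explosion sound and particles, then deals radial explosive damage with falloff, ignoring itself.
; HealthComponent's OnDeath also calls Attack, and the CanAttack flag blocks repeat blasts.
; The mesh is hidden after the blast, and a zero-length Delay precedes destroying the actor.
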(event OnDeath(HealthComponent)
  (Class|DroneBase|Attack))

(event EventAttack
  (if (Variables|Default|GetbCanAttack)
    (Audio|PlaySoundatLocation "/Game/StarterContent/Audio/Explosion_Cue.Explosion_Cue" (Transformation|GetActorLocation) "0, 0, 0" 1.0 1.0 0.0 0 0 0)
    (Effects|SpawnEmitteratLocation (Variables|Default|GetExplotionParticle) (Transformation|GetActorLocation) "0, 0, 0" "5.000000,5.000000,5.000000")
    (Class|GameplayStatics|ApplyRadialDamagewithFalloff (Variables|Default|GetMaxDamage) (Variables|Default|GetMinimumDamage) (Transformation|GetActorLocation) (Variables|Default|GetInnerRadius) (Variables|Default|GetOuterRadius) 1.0 "/Game/ShooterTest/Misc/Damage/DamageType_Explosive.DamageType_Explosive_C" (Utilities|Array|MakeArray self) self (Pawn|GetController) "ECC_Visibility")
    (Rendering|SetVisibility (Variables|Character|GetMesh) false false)
    (Variables|Default|SetbCanAttack false)
    (Utilities|FlowControl|Delay 0.0)
    (Actor|DestroyActor)))

(fn ConstructionScript)