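; BP_RangeEnemy is an armed enemy character that attacks with a child-actor weapon and awards score when killed.
; On possession it registers itself as the weapon's user, and Attack calls the OnFire dispatcher while attacking is allowed.
; Death disables attacks, removes the weapon, adds score through BP_GameMode and destroys the actor after a delay.
; Lethal damage pushes the mesh's head bone away from the damage causer.
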(event EventPossessed
  (params (NewController :type Controller%20Object%20Reference))
  (bind _asbp_weapon (Utilities|Casting|CastToBP_Weapon (Variables|/Script/Engine.ChildActorComponent|GetChildActor (Variables|Default|GetWeapon))))
  (Class|WeaponBase|SetUser _asbp_weapon self))

(event EventAttack
  (if (Variables|Default|GetbCanAttack)
    (Default|CallOnFire)))

(event EventDie
  (Variables|Default|SetbCanAttack false)
  (Components|DestroyComponent (Variables|Default|GetWeapon))
  (bind _asbp_game_mode (Utilities|Casting|CastToBP_GameMode (Game|GetGameMode)))
  (Default|AddScore _asbp_game_mode (Variables|Default|GetScoreToAdd))
  (Utilities|FlowControl|Delay 5.0)
  (Actor|DestroyActor))

(event Game|Damage|EventAnyDamage
  (params (Damage :type Float%20%28single-precision%29) (DamageType :type Damage%20Type%20Object%20Reference) (InstigatedBy :type Controller%20Object%20Reference) (DamageCauser :type Actor%20Object%20Reference))
  (if (<= (Class|CharacterBase|GetHealth) 0.0)
    (Utilities|IsValid DamageCauser
      (:Is%20Valid
        (Physics|AddImpulse (Variables|Character|GetMesh) (* (- (Transformation|GetActorLocation) (Transformation|GetActorLocation DamageCauser)) 5e+01) "Head" false)))))

(fn ConstructionScript)